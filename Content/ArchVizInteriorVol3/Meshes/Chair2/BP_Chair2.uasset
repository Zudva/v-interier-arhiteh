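; Interactive chair actor for an interior archviz scene that lets the player cycle material finishes on three chair meshes at once.
; Overlapping the Box enables input and toggles the PressE prompt, and leaving disables input and toggles it again.
; Each E press advances a looping MultiGate through five steps, each swapping one of two material slots, so the other slot keeps its current material.
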(event OnComponentBeginOverlap(Box)
  (params (OverlappedComponent :type Primitive%20Component%20Object%20Reference) (OtherActor :type Actor%20Object%20Reference) (OtherComp :type Primitive%20Component%20Object%20Reference) (OtherBodyIndex :type Integer) (bFromSweep :type Boolean) (SweepResult :type Hit%20Result%20Structure%20%28by%20ref%29))
  (Input|EnableInput (Game|GetPlayerController 0))
  (Rendering|ToggleVisibility (Variables|Default|GetPress%20E) false))

(event OnComponentEndOverlap(Box)
  (params (OverlappedComponent :type Primitive%20Component%20Object%20Reference) (OtherActor :type Actor%20Object%20Reference) (OtherComp :type Primitive%20Component%20Object%20Reference) (OtherBodyIndex :type Integer))
  (Input|DisableInput (Game|GetPlayerController 0))
  (Rendering|ToggleVisibility (Variables|Default|GetPress%20E) false))

(event EventBeginPlay)

(event Collision|EventActorBeginOverlap
  (params (OtherActor :type Actor%20Object%20Reference)))

(event EventTick
  (params (DeltaSeconds :type Float%20%28single-precision%29)))

(event Input|KeyboardEvents|E
  (params (Key :type Key%20Structure :default "None"))
  (bind _chair (Variables|Default|GetChair))
  (:Pressed
    (Utilities|FlowControl|MultiGate false true -1
      (:Out%200
        (Rendering|Material|SetMaterial _chair 0 "/Game/ArchVizInteriorVol3/Materials/M_Chair1.M_Chair1"))
      (:Out%201
        (Rendering|Material|SetMaterial _chair 1 "/Game/ArchVizInteriorVol3/Meshes/Chair2/M_Chair_2_seat2.M_Chair_2_seat2"))
      (:Out%202
        (Rendering|Material|SetMaterial _chair 1 "/Game/ArchVizInteriorVol3/Meshes/Chair2/M_Chair_2_seat3.M_Chair_2_seat3"))
      (:Out%203
        (Rendering|Material|SetMaterial _chair 0 "/Game/ArchVizInteriorVol3/Meshes/Chair2/M_Tabletop_3.M_Tabletop_3"))
      (:Out%204
        (Rendering|Material|SetMaterial _chair 0 "/Game/ArchVizInteriorVol3/Meshes/Chair2/M_Tabletop_4.M_Tabletop_4")))))

(fn ConstructionScript)